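; Falling enemy for a typing game, held by one to three colored balloons with unique random letters, that ends the game if it lands alive.
; Matching key presses queue balloons, which Tick pops through five copied slots (A–E) so delayed pop animations can overlap.
; Losing every letter kills it: score and high-score text update, and a timeline rotates the body and alters fall speed until it hits the floor and is destroyed.
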(event Custom|Key_Pressed
  (params (Key :type Key%20Structure :default "AnyKey"))
  (bind _key_list (Variables|Lists|GetKey_list))
  (bind _alphabets (Variables|BalloonInfo|GetAlphabets))
  (bind _alphabet_list (Variables|Lists|GetAlphabet_list))
  (bind _returnvalue (Utilities|Array|FindItem _key_list Key))
  (bind _item (Utilities|Array|Get(acopy) _alphabet_list _returnvalue))
  (bind _returnvalue_2 (Utilities|Array|FindItem _alphabets _item))
  ;[1 1 1] A~Z 중 하나인가?
  (if (>= _returnvalue 0)
    ;[1 1 1] 해당 글자의 풍선이 있는가?
    (if (>= _returnvalue_2 0)
      ;[1 1 1] 터뜨리는 풍선 대기열에 추가
      (Utilities|Array|Add (Variables|PoppingBalloon|GetPop_Balloon_Index) _returnvalue_2)
      (bind _ascharacter_blueprint (Utilities|Casting|CastToCharacter_Blueprint (Game|Player|GetPlayerPawn 0)))
      (Variables|/Game/Blueprints/Character_Blueprint.Character_Blueprint_C|SetSuccess_Count _ascharacter_blueprint 1))))

(event EventBeginPlay
  (bind _alphabets (Variables|BalloonInfo|GetAlphabets))
  (Utilities|FlowControl|Sequence
    (:then_0
      ;[1 1 1] 풍선 개수
      (Variables|Balloon_Info|SetBall_Num (+ (Math|Random|RandomInteger 3) 1))
      (while (> (Variables|Balloon_Info|GetBall_Num) (Variables|Default|GetLooping))
        ;[1 1 1] 풍선 추가
        (bind _returnvalue (AddComponent|AddPaperFlipbookComponent true (Math|Transform|MakeTransform "0,-10.000000,320.000000" "0, 0, 0" "1,1,1")))
        (Sprite|SetFlipbook _returnvalue "/Game/Animations/Balloon_Anim.Balloon_Anim")
        (Transformation|AttachComponentToComponent _returnvalue (Variables|Default|GetBody) "None" "KeepRelative" "KeepRelative" "KeepRelative" true)
        (switch int (Variables|Default|GetLooping)
          (:0
            _)
          (:1
            (Variables|Balloon_Info|SetBall_Rot "45.000000, 0,0.000000")
            (Variables|Balloon_Info|SetBall_Loc "-109.000000,-10.000000,300.000000"))
          (:2
            (Variables|Balloon_Info|SetBall_Rot "-45.000000, 0,0.000000")
            (Variables|Balloon_Info|SetBall_Loc "111.000000,-10.000000,300.000000")))
        (Transformation|SetRelativeLocationAndRotation _returnvalue (Variables|Balloon_Info|GetBall_Loc) (Variables|Balloon_Info|GetBall_Rot) false false)
        (bind _returnvalue_2 (Utilities|Array|Add (Variables|Balloon_Info|GetBalloons) _returnvalue))
        ;[1 1 1] 텍스트 컴포넌트 추가
        (bind _returnvalue_3 (AddComponent|AddTextRenderComponent true))
        (Transformation|AttachComponentToComponent _returnvalue_3 (Utilities|Array|Get(acopy) (Variables|Balloon_Info|GetBalloons) _returnvalue_2) "None" "KeepRelative" "KeepRelative" "KeepRelative" true)
        (Transformation|SetRelativeLocationAndRotation _returnvalue_3 "-27.000000,10.000000,50.000000" "0.000000,90.000000,0.000000" false false)
        (Transformation|SetRelativeScale3D _returnvalue_3 "1.000000,3.500000,3.500000")
        ;[1 1 1] 텍스트 설정
        (Variables|BalloonInfo|SetAlphabet_Index (Math|Random|RandomInteger 26))
        (while (> (Utilities|Array|FindItem _alphabets (Utilities|Array|Get(acopy) (Variables|Lists|GetAlphabet_list) (Variables|BalloonInfo|GetAlphabet_Index))) -1)
          (Variables|BalloonInfo|SetAlphabet_Index (Math|Random|RandomInteger 26)))
        (bind _returnvalue_4 (Utilities|Array|Add _alphabets (Utilities|Array|Get(acopy) (Variables|Lists|GetAlphabet_list) (Variables|BalloonInfo|GetAlphabet_Index))))
        (Rendering|Components|TextRender|SetText _returnvalue_3 (Utilities|Array|Get(acopy) (Variables|BalloonInfo|GetAlphabets) _returnvalue_4))
        (Rendering|Components|TextRender|SetTextRenderColor :self _returnvalue_3)
        ;[1 1 1] 풍선 색 설정
        (Sprite|SetSpriteColor _returnvalue (Utilities|Array|Get(acopy) (Variables|Lists|GetBall_Color) (Variables|BalloonInfo|GetAlphabet_Index)))
        (Variables|Default|SetLooping (+ (Variables|Default|GetLooping) 1))))
    (:then_1
      ;[1 1 1] 레퍼런스 세팅
      (bind _outactors (Actor|GetAllActorsOfClass "/Game/Blueprints/Floor_Blueprint.Floor_Blueprint_C"))
      (Variables|References|SetFloor (Utilities|Array|Get(acopy) _outactors))
      (bind _outactors_2 (Actor|GetAllActorsOfClass "/Game/Blueprints/Score_Blueprint.Score_Blueprint_C"))
      (Variables|References|SetScore (Utilities|Array|Get(acopy) _outactors_2))
      (bind _outactors_3 (Actor|GetAllActorsOfClass "/Game/Blueprints/Character_Blueprint.Character_Blueprint_C"))
      (Variables|References|SetCharacter (Utilities|Array|Get(acopy) _outactors_3))
      (bind _outactors_4 (Actor|GetAllActorsOfClass "/Game/Blueprints/Highest_Score_Blueprint.Highest_Score_Blueprint_C"))
      (Variables|References|SetHS_Score (Utilities|Array|Get(acopy) _outactors_4)))))

(event EventTick
  (params (DeltaSeconds :type Float%20%28single-precision%29))
  (bind _returnvalue (Transformation|GetActorLocation))
  (bind _body (Variables|Default|GetBody))
  (bind _pop_balloon_index (Variables|PoppingBalloon|GetPop_Balloon_Index))
  (bind _in_charge (Variables|PoppingBalloon|GetIn_Charge))
  (bind _pop_balloon_index_2 (Variables|PoppingBalloon|GetPop_Balloon_Index))
  (bind _pop_balloon_index_3 (Variables|PoppingBalloon|GetPop_Balloon_Index))
  (bind _pop_balloon_index_4 (Variables|PoppingBalloon|GetPop_Balloon_Index))
  (bind _pop_balloon_index_5 (Variables|PoppingBalloon|GetPop_Balloon_Index))
  (bind _score (Variables|References|GetScore))
  (bind _score_2 (Variables|/Game/Blueprints/Score_Blueprint.Score_Blueprint_C|GetScore _score))
  (Utilities|FlowControl|Sequence
    (:then_0
      ;[1 1 1] 자동 낙하
      (bind _sweephitresult (Transformation|SetActorLocation (Math|Vector|MakeVector (.x _returnvalue) (.y _returnvalue) (- (.z _returnvalue) (+ (Variables|/Game/Blueprints/Character_Blueprint.Character_Blueprint_C|GetFall_Speed (Variables|References|GetCharacter)) (Variables|Default|GetLocal_Fall_Speed)))) true false))
      ;[1 1 1] 바닥에 닿았을 때
      (if (== (.hitactor _sweephitresult) (Variables|References|GetFloor))
        (if (Variables|Default|GetIsDead)
          ;[1 1 1] 죽은 상태이면
          (Utilities|FlowControl|DoOnce false
            (:Completed
              (Sprite|SetFlipbook _body "/Game/Animations/Mob_Re_Dead_Anim.Mob_Re_Dead_Anim")
              (Audio|PlaySoundatLocation "/Game/Sounds/Body_Fall_Sound.Body_Fall_Sound" (Transformation|GetWorldLocation _body) "0, 0, 0" 0.4 (Math|Random|RandomFloatinRange 0.8 1.2))
              (Utilities|FlowControl|Delay 0.55)
              (Actor|DestroyActor)))
          (else
            ;[1 1 1] 산 상태이면 - 게임 오버
            (Variables|Default|SetIsDead true) ; 이벤트가 래피드 호출되는 것을 막기 위한 거짓 죽음
            (Default|GameOver (Variables|References|GetCharacter))))))
    (:then_1
      ;[1 1 1] 풍선 터뜨리기
      (if (!= 0 (Utilities|Array|Length (Variables|PoppingBalloon|GetPop_Balloon_Index)))
        (if (== (Utilities|Array|FindItem (Variables|PoppingBalloon|GetIn_Charge) "A") -1)
          (Utilities|Array|Add _in_charge (Utilities|String|MakeLiteralString "A"))
          (bind _output_get (Variables|Index_of_Thread|SetIndex_A (Utilities|Array|Get(acopy) _pop_balloon_index_2)))
          (Utilities|Array|RemoveItem _pop_balloon_index_2 _output_get)
          (Audio|PlaySoundatLocation "/Game/Sounds/Pop_Sound.Pop_Sound" (Transformation|GetWorldLocation (Utilities|Array|Get(acopy) (Variables|Balloon_Info|GetBalloons) _output_get)) "0, 0, 0" 0.4 (Math|Random|RandomFloatinRange 0.8 1.2))
          (Sprite|SetFlipbook (Utilities|Array|Get(acopy) (Variables|Balloon_Info|GetBalloons) _output_get) "/Game/Animations/Ballon_Pop_Anim.Ballon_Pop_Anim")
          (Utilities|Array|RemoveIndex (Variables|BalloonInfo|GetAlphabets) (Variables|Index_of_Thread|GetIndex_A))
          (Utilities|FlowControl|Delay 0.26)
          (Components|DestroyComponent (Components|GetChildComponent (Utilities|Array|Get(acopy) (Variables|Balloon_Info|GetBalloons) _output_get) 0))
          (Utilities|Array|RemoveIndex (Variables|Balloon_Info|GetBalloons) (Variables|Index_of_Thread|GetIndex_A))
          (Utilities|Array|RemoveItem (Variables|PoppingBalloon|GetIn_Charge) (Utilities|String|MakeLiteralString "A"))
          (elif (== (Utilities|Array|FindItem (Variables|PoppingBalloon|GetIn_Charge) "B") -1)
            (Utilities|Array|Add _in_charge (Utilities|String|MakeLiteralString "B"))
            (bind _output_get_2 (Variables|IndexOfThread|SetIndex_B (Utilities|Array|Get(acopy) _pop_balloon_index_3)))
            (Utilities|Array|RemoveItem _pop_balloon_index_3 _output_get_2)
            (Audio|PlaySoundatLocation "/Game/Sounds/Pop_Sound.Pop_Sound" (Transformation|GetWorldLocation (Utilities|Array|Get(acopy) (Variables|Balloon_Info|GetBalloons) _output_get_2)) "0, 0, 0" 0.4 (Math|Random|RandomFloatinRange 0.8 1.2))
            (Sprite|SetFlipbook (Utilities|Array|Get(acopy) (Variables|Balloon_Info|GetBalloons) _output_get_2) "/Game/Animations/Ballon_Pop_Anim.Ballon_Pop_Anim")
            (Utilities|Array|RemoveIndex (Variables|BalloonInfo|GetAlphabets) (Variables|IndexOfThread|GetIndex_B))
            (Utilities|FlowControl|Delay 0.26)
            (Components|DestroyComponent (Components|GetChildComponent (Utilities|Array|Get(acopy) (Variables|Balloon_Info|GetBalloons) _output_get_2) 0))
            (Utilities|Array|RemoveIndex (Variables|Balloon_Info|GetBalloons) (Variables|IndexOfThread|GetIndex_B))
            (Utilities|Array|RemoveItem (Variables|PoppingBalloon|GetIn_Charge) (Utilities|String|MakeLiteralString "B"))
            (elif (== (Utilities|Array|FindItem (Variables|PoppingBalloon|GetIn_Charge) "C") -1)
              (Utilities|Array|Add _in_charge (Utilities|String|MakeLiteralString "C"))
              (bind _output_get_3 (Variables|IndexOfThread|SetIndex_C (Utilities|Array|Get(acopy) _pop_balloon_index_4)))
              (Utilities|Array|RemoveItem _pop_balloon_index_4 _output_get_3)
              (Audio|PlaySoundatLocation "/Game/Sounds/Pop_Sound.Pop_Sound" (Transformation|GetWorldLocation (Utilities|Array|Get(acopy) (Variables|Balloon_Info|GetBalloons) _output_get_3)) "0, 0, 0" 0.4 (Math|Random|RandomFloatinRange 0.8 1.2))
              (Sprite|SetFlipbook (Utilities|Array|Get(acopy) (Variables|Balloon_Info|GetBalloons) _output_get_3) "/Game/Animations/Ballon_Pop_Anim.Ballon_Pop_Anim")
              (Utilities|Array|RemoveIndex (Variables|BalloonInfo|GetAlphabets) (Variables|IndexOfThread|GetIndex_C))
              (Utilities|FlowControl|Delay 0.26)
              (Components|DestroyComponent (Components|GetChildComponent (Utilities|Array|Get(acopy) (Variables|Balloon_Info|GetBalloons) _output_get_3) 0))
              (Utilities|Array|RemoveIndex (Variables|Balloon_Info|GetBalloons) (Variables|IndexOfThread|GetIndex_C))
              (Utilities|Array|RemoveItem (Variables|PoppingBalloon|GetIn_Charge) (Utilities|String|MakeLiteralString "C"))
              (elif (== (Utilities|Array|FindItem (Variables|PoppingBalloon|GetIn_Charge) "D") -1)
                (Utilities|Array|Add _in_charge (Utilities|String|MakeLiteralString "D"))
                (bind _output_get_4 (Variables|IndexOfThread|SetIndex_D (Utilities|Array|Get(acopy) _pop_balloon_index_5)))
                (Utilities|Array|RemoveItem _pop_balloon_index_5 _output_get_4)
                (Audio|PlaySoundatLocation "/Game/Sounds/Pop_Sound.Pop_Sound" (Transformation|GetWorldLocation (Utilities|Array|Get(acopy) (Variables|Balloon_Info|GetBalloons) _output_get_4)) "0, 0, 0" 0.4 (Math|Random|RandomFloatinRange 0.8 1.2))
                (Sprite|SetFlipbook (Utilities|Array|Get(acopy) (Variables|Balloon_Info|GetBalloons) _output_get_4) "/Game/Animations/Ballon_Pop_Anim.Ballon_Pop_Anim")
                (Utilities|Array|RemoveIndex (Variables|BalloonInfo|GetAlphabets) (Variables|IndexOfThread|GetIndex_D))
                (Utilities|FlowControl|Delay 0.26)
                (Components|DestroyComponent (Components|GetChildComponent (Utilities|Array|Get(acopy) (Variables|Balloon_Info|GetBalloons) _output_get_4) 0))
                (Utilities|Array|RemoveIndex (Variables|Balloon_Info|GetBalloons) (Variables|IndexOfThread|GetIndex_D))
                (Utilities|Array|RemoveItem (Variables|PoppingBalloon|GetIn_Charge) (Utilities|String|MakeLiteralString "D"))
                (elif (== (Utilities|Array|FindItem (Variables|PoppingBalloon|GetIn_Charge) "E") -1)
                  (Utilities|Array|Add _in_charge (Utilities|String|MakeLiteralString "E"))
                  (bind _output_get_5 (Variables|IndexOfThread|SetIndex_E (Utilities|Array|Get(acopy) _pop_balloon_index)))
                  (Utilities|Array|RemoveItem _pop_balloon_index _output_get_5)
                  (Audio|PlaySoundatLocation "/Game/Sounds/Pop_Sound.Pop_Sound" (Transformation|GetWorldLocation (Utilities|Array|Get(acopy) (Variables|Balloon_Info|GetBalloons) _output_get_5)) "0, 0, 0" 0.4 (Math|Random|RandomFloatinRange 0.8 1.2))
                  (Sprite|SetFlipbook (Utilities|Array|Get(acopy) (Variables|Balloon_Info|GetBalloons) _output_get_5) "/Game/Animations/Ballon_Pop_Anim.Ballon_Pop_Anim")
                  (Utilities|Array|RemoveIndex (Variables|BalloonInfo|GetAlphabets) (Variables|IndexOfThread|GetIndex_E))
                  (Utilities|FlowControl|Delay 0.26)
                  (Components|DestroyComponent (Components|GetChildComponent (Utilities|Array|Get(acopy) (Variables|Balloon_Info|GetBalloons) _output_get_5) 0))
                  (Utilities|Array|RemoveIndex (Variables|Balloon_Info|GetBalloons) (Variables|IndexOfThread|GetIndex_E))
                  (Utilities|Array|RemoveItem (Variables|PoppingBalloon|GetIn_Charge) (Utilities|String|MakeLiteralString "E"))
                  (else
                    (Development|PrintString "Warning! Need More Space" true true "(R=1.000000,G=0.015914,B=0.000000,A=1.000000)" 1e+01)))))))))
    (:then_2
      ;[1 1 1] 사망
      (if (not (Variables|Default|GetIsDead))
        (if (== (Utilities|Array|Length (Variables|BalloonInfo|GetAlphabets)) 0)
          (Variables|Default|SetIsDead true)
          (Utilities|Array|RemoveItem (Variables|/Game/Blueprints/Character_Blueprint.Character_Blueprint_C|GetMob_Re (Variables|References|GetCharacter)) self)
          (Default|ScoreUpdate (Variables|References|GetScore) 1)
          (if (>= _score_2 (Variables|/Game/Blueprints/Character_Blueprint.Character_Blueprint_C|GetHS_Original (Variables|References|GetCharacter)))
            (Rendering|Components|TextRender|SetText (Variables|/Game/Blueprints/Highest_Score_Blueprint.Highest_Score_Blueprint_C|GetScore (Variables|References|GetHS_Score)) (Utilities|Text|ToText(Integer) _score_2))
            (bind (_direction _roll _falling_speed) (Timeline|Dead_Rotation Play)
              (:Update
                (Transformation|SetRelativeRotation (Variables|Default|GetBody) (Math|Rotator|MakeRotator _roll 0.0 0.0) false false)
                (Variables|Default|SetLocal_Fall_Speed _falling_speed)))
            (else
              (Timeline|Dead_Rotation Play))))))))

(fn ConstructionScript)