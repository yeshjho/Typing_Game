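; Score actor that keeps the running score, shows it on a text render and drives difficulty progression.
; Score_Update adds points, then checks score tiers from 11 upward, each firing once through a DoOnce.
; A new tier calls SpdSpRate, which sets the Character's SpawnChance, adds to its cumulative FallSpeed and updates its widget with a "Level Up" speed notice and the spawn value.
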(event Custom|Score_Update
  (params (Score_Add :type Integer))
  (bind _output_get (Variables|Default|SetScore (+ Score_Add (Variables|Default|GetScore))))
  (Rendering|Components|TextRender|SetText (Variables|Default|GetTextRender) (Utilities|Text|ToText(Integer) _output_get))
  (if (and (>= (Variables|Default|GetScore) 11) (<= (Variables|Default|GetScore) 30))
    (Utilities|FlowControl|DoOnce false
      (:Completed
        (CallFunction|SpdSpRate 100 1.5)))
    (elif (and (>= (Variables|Default|GetScore) 31) (<= (Variables|Default|GetScore) 50))
      (Utilities|FlowControl|DoOnce false
        (:Completed
          (CallFunction|SpdSpRate 80 2.5)))
      (elif (and (>= (Variables|Default|GetScore) 51) (<= (Variables|Default|GetScore) 100))
        (Utilities|FlowControl|DoOnce false
          (:Completed
            (CallFunction|SpdSpRate 60 3.0)))
        (elif (and (>= (Variables|Default|GetScore) 101) (<= (Variables|Default|GetScore) 200))
          (Utilities|FlowControl|DoOnce false
            (:Completed
              (CallFunction|SpdSpRate 50 3.5)))
          (elif (and (>= (Variables|Default|GetScore) 201) (<= (Variables|Default|GetScore) 500))
            (Utilities|FlowControl|DoOnce false
              (:Completed
                (CallFunction|SpdSpRate 45 4.0)))
            (elif (and (>= (Variables|Default|GetScore) 501) (<= (Variables|Default|GetScore) 1000))
              (Utilities|FlowControl|DoOnce false
                (:Completed
                  (CallFunction|SpdSpRate 40 5.0)))
              (elif (>= (Variables|Default|GetScore) 1001)
                (Utilities|FlowControl|DoOnce false
                  (:Completed
                    (CallFunction|SpdSpRate 30 8.0)))))))))))

(fn ConstructionScript)

(fn SpdSpRate
  (params (SpawnRate :type Integer) (FallSpeed :type Float%20%28single-precision%29))
  (bind _character (Variables|Default|GetCharacter))
  (bind _default_widget (Variables|/Game/Blueprints/Character_Blueprint.Character_Blueprint_C|GetDefault_Widget _character))
  (Variables|/Game/Blueprints/Character_Blueprint.Character_Blueprint_C|SetSpawn_Chance _character SpawnRate)
  (Variables|/Game/Blueprints/Character_Blueprint.Character_Blueprint_C|SetFall_Speed _character (+ FallSpeed (Variables|/Game/Blueprints/Character_Blueprint.Character_Blueprint_C|GetFall_Speed _character)))
  (Default|SpeedUpdate _default_widget FallSpeed "Level Up")
  (Default|SpawnUpdate _default_widget SpawnRate))