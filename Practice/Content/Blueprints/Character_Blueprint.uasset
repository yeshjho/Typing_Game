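; Player character that runs a balloon-typing game, from option and menu screens through pause, game over and restart.
; Tick randomly spawns Mob_Re balloons and gathers those with letters remaining into MobRe.
; Key presses go to every listed balloon; a miss raises FallSpeed, while a hit clears the list for Tick to rebuild.
; Game over stops the ambient sound and saves a new high score to a slot, which Start reloads.
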(event Custom|Game%20Over
  (bind _returnvalue (Game|GetPlayerController 0))
  (bind _score (Variables|Default|GetScore))
  (bind _score_2 (Variables|/Game/Blueprints/Score_Blueprint.Score_Blueprint_C|GetScore _score))
  ;[1 1 1] 게임 오버 화면 띄우기
  (bind _returnvalue_2 (UserInterface|CreateWidget "/Game/Widgets/Game_Over_Widget.Game_Over_Widget_C" _returnvalue))
  (bind _output_get (Variables|Widgets|SetGame_Over_Widget _returnvalue_2))
  (UserInterface|Viewport|AddtoViewport _output_get 900)
  (Input|SetInputModeUIOnly _returnvalue _returnvalue_2 "DoNotLock")
  (Variables|/Script/Engine.PlayerController|SetbShowMouseCursor _returnvalue true)
  (Variables|Default|SetIsGameOver true)
  (Variables|Default|SetFall_Speed 0.0)
  (bind _outactors (Actor|GetAllActorsOfClass "/Script/Engine.AmbientSound"))
  (Audio|Components|Audio|Stop (Variables|/Script/Engine.AmbientSound|GetAudioComponent (Utilities|Array|Get(acopy) _outactors)))
  (Utilities|FlowControl|Delay 0.1)
  (Audio|PlaySound2D "/Game/Sounds/Game_Over_Sound.Game_Over_Sound" 0.1)
  ;[1 1 1] 최고 기록 저장
  (if (> _score_2 (Variables|Default|GetHS_Original))
    (bind _returnvalue_3 (SaveGame|CreateSaveGameObject "/Game/SaveGame/Save_Game_1_Blueprint.Save_Game_1_Blueprint_C"))
    (Variables|/Game/SaveGame/Save_Game_1_Blueprint.Save_Game_1_Blueprint_C|SetHighest_Score _returnvalue_3 _score_2)
    (SaveGame|SaveGametoSlot _returnvalue_3 "Slot_1")))

(event Custom|Restart
  (bind _returnvalue (Game|GetPlayerController 0))
  (Utilities|FlowControl|Sequence
    (:then_0
      (Utilities|FlowControl|Sequence
        (:then_0
          (Utilities|FlowControl|DoOnce false
            (:Completed
              (bind _returnvalue_2 (UserInterface|CreateWidget "/Game/Widgets/Default_Widget.Default_Widget_C" (Game|GetPlayerController 0)))
              (bind _output_get (Variables|Widgets|SetDefault_Widget _returnvalue_2))
              (UserInterface|Viewport|AddtoViewport _output_get 50))))
        (:then_1
          (Variables|Default|SetIsGameOver false))
        (:then_2
          ;[1 1 1] 최고 기록 띄우기
          (bind _returnvalue_3 (SaveGame|LoadGamefromSlot "Slot_1"))
          (bind _assave_game_1_blueprint (Utilities|Casting|CastToSave_Game_1_Blueprint _returnvalue_3))
          (bind _output_get_2 (Variables|Default|SetHS_Original (Variables|/Game/SaveGame/Save_Game_1_Blueprint.Save_Game_1_Blueprint_C|GetHighest_Score _assave_game_1_blueprint)))
          (Rendering|Components|TextRender|SetText (Variables|/Game/Blueprints/Highest_Score_Blueprint.Highest_Score_Blueprint_C|GetScore (Variables|Default|GetHighest_Score_Actor)) (Utilities|Text|ToText(Integer) _output_get_2)))))
    (:then_1
      ;[1 1 1] 남아 있던 몹 제거
      (for _array_element (Variables|Default|GetMob_Re)
        (Actor|DestroyActor _array_element)))
    (:then_2
      ;[1 1 1] 게임 오버 화면 제거
      (Input|SetInputModeGameOnly _returnvalue)
      (Variables|/Script/Engine.PlayerController|SetbShowMouseCursor _returnvalue false)
      (Widget|RemovefromParent (Variables|Widgets|GetGame_Over_Widget))
      (Variables|/Game/Widgets/Default_Widget.Default_Widget_C|SetSpeed (Variables|Widgets|GetDefault_Widget) 1.0)
      (Utilities|Array|Clear (Variables|/Game/Widgets/Default_Widget.Default_Widget_C|GetReasons (Variables|Widgets|GetDefault_Widget)))
      (Rendering|Components|TextRender|SetText (Variables|/Game/Widgets/Default_Widget.Default_Widget_C|GetSpawn_Rate_Text (Variables|Widgets|GetDefault_Widget)) "1/120 per tick")
      (Default|SpeedUpdate (Variables|Widgets|GetDefault_Widget) 0.0)
      (Rendering|Components|TextRender|SetText (Variables|/Game/Widgets/Default_Widget.Default_Widget_C|GetReason_F (Variables|Widgets|GetDefault_Widget)) "")
      (Utilities|Array|Clear (Variables|/Game/Widgets/Default_Widget.Default_Widget_C|GetReasons (Variables|Widgets|GetDefault_Widget))))
    (:then_3
      (bind _outactors (Actor|GetAllActorsOfClass "/Script/Engine.AmbientSound"))
      (Audio|Components|Audio|Play (Variables|/Script/Engine.AmbientSound|GetAudioComponent (Utilities|Array|Get(acopy) _outactors)) 0.0)
      (Utilities|Array|Clear (Variables|Default|GetMob_Re))
      (Variables|Default|SetFall_Speed 1.0)
      (Variables|/Game/Blueprints/Score_Blueprint.Score_Blueprint_C|SetScore (Variables|Default|GetScore) 0)
      (Default|ScoreUpdate (Variables|Default|GetScore))
      (Variables|Default|SetSpawn_Chance 120))))

(event Custom|Start
  (Utilities|FlowControl|Sequence
    (:then_0
      (Utilities|FlowControl|DoOnce false
        (:Completed
          (bind _returnvalue (UserInterface|CreateWidget "/Game/Widgets/Default_Widget.Default_Widget_C" (Game|GetPlayerController 0)))
          (bind _output_get (Variables|Widgets|SetDefault_Widget _returnvalue))
          (UserInterface|Viewport|AddtoViewport _output_get 50))))
    (:then_1
      (Variables|Default|SetIsGameOver false))
    (:then_2
      ;[1 1 1] 최고 기록 띄우기
      (bind _returnvalue_2 (SaveGame|LoadGamefromSlot "Slot_1"))
      (bind _assave_game_1_blueprint (Utilities|Casting|CastToSave_Game_1_Blueprint _returnvalue_2))
      (bind _output_get_2 (Variables|Default|SetHS_Original (Variables|/Game/SaveGame/Save_Game_1_Blueprint.Save_Game_1_Blueprint_C|GetHighest_Score _assave_game_1_blueprint)))
      (Rendering|Components|TextRender|SetText (Variables|/Game/Blueprints/Highest_Score_Blueprint.Highest_Score_Blueprint_C|GetScore (Variables|Default|GetHighest_Score_Actor)) (Utilities|Text|ToText(Integer) _output_get_2)))))

(event Custom|Hovered
  (params (Image :type Image%20Object%20Reference))
  (Utilities|FlowControl|FlipFlop
    (:A
      (bind _opacity (Timeline|Opacity_Timeline Play)
        (:Update
          (for _array_element (Variables|/Game/Widgets/Option_Widget.Option_Widget_C|GetKeyboards (Variables|Widgets|GetOption_Widget))
            (if (!= _array_element Image)
              (Class|Image|SetOpacity _array_element _opacity))))))
    (:B
      (Timeline|Opacity_Timeline Reverse))))

(event Custom|Resume
  (bind _returnvalue (Game|GetPlayerController 0))
  (Input|SetInputModeGameOnly _returnvalue)
  (Variables|/Script/Engine.PlayerController|SetbShowMouseCursor _returnvalue false)
  (Game|SetGamePaused false)
  (Variables|Default|SetIsPaused false)
  (Widget|RemovefromParent (Variables|Widgets|GetPaused_Widget)))

(event Custom|Create_Default_Widget
  (bind _returnvalue (UserInterface|CreateWidget "/Game/Widgets/Default_Widget.Default_Widget_C" (Game|GetPlayerController 0)))
  (bind _output_get (Variables|Widgets|SetDefault_Widget _returnvalue))
  (UserInterface|Viewport|AddtoViewport _output_get 50))

(event Custom|Pause
  (bind _returnvalue (Game|GetPlayerController 0))
  (if (not (Variables|Default|GetIsPaused))
    (Variables|Default|SetIsPaused true)
    (bind _returnvalue_2 (UserInterface|CreateWidget "/Game/Widgets/Paused_Widget.Paused_Widget_C" _returnvalue))
    (bind _output_get (Variables|Widgets|SetPaused_Widget _returnvalue_2))
    (UserInterface|Viewport|AddtoViewport _output_get 5)
    (Input|SetInputModeUIOnly _returnvalue _output_get "DoNotLock")
    (Variables|/Script/Engine.PlayerController|SetbShowMouseCursor _returnvalue true)
    (Game|SetGamePaused true)))

(event Custom|Create_Main_Menu_Widget
  (bind _returnvalue (Game|GetPlayerController 0))
  ;[1 1 1] 메인 메뉴 띄우기
  (Game|SetGamePaused true)
  (bind _returnvalue_2 (UserInterface|CreateWidget "/Game/Widgets/Main_Menu_Widget.Main_Menu_Widget_C" _returnvalue))
  (bind _output_get (Variables|Widgets|SetMain_Menu_Widget _returnvalue_2))
  (UserInterface|Viewport|AddtoViewport _output_get 90)
  (Input|SetInputModeUIOnly _returnvalue _output_get "DoNotLock")
  (Variables|/Script/Engine.PlayerController|SetbShowMouseCursor _returnvalue true)
  (Development|ExecuteConsoleCommand "r.SetRes 1920x1080f"))

(event EventBeginPlay
  (bind _returnvalue (Game|GetPlayerController 0))
  (Game|SetGamePaused true)
  (bind _returnvalue_2 (UserInterface|CreateWidget "/Game/Widgets/Option_Widget.Option_Widget_C" _returnvalue))
  (bind _output_get (Variables|Widgets|SetOption_Widget _returnvalue_2))
  (UserInterface|Viewport|AddtoViewport _output_get 90)
  (Input|SetInputModeUIOnly _returnvalue _output_get "DoNotLock")
  (Variables|/Script/Engine.PlayerController|SetbShowMouseCursor _returnvalue true))

(event EventTick
  (params (DeltaSeconds :type Float%20%28single-precision%29))
  (if (not (Variables|Default|GetIsGameOver))
    (Utilities|FlowControl|Sequence
      (:then_0
        ;[1 1 1] Mob_Re 리스트 생성(액터 생성 시 추가하지 않는 이유는 Remove할 때 블루프린트 클래스로 해서 화면에 있는 모든 액터가 사라짐)
        (bind _outactors (Actor|GetAllActorsOfClass "/Game/Blueprints/Mob_Re_Blueprint.Mob_Re_Blueprint_C"))
        (for _array_element _outactors
          (if (!= (Utilities|Array|Length (Variables|/Game/Blueprints/Mob_Re_Blueprint.Mob_Re_Blueprint_C|GetAlphabets _array_element)) 0)
            (Utilities|Array|AddUnique (Variables|Default|GetMob_Re) _array_element))))
      (:then_1
        ;[1 1 1] 몹 생성
        (if (== (Math|Random|RandomInteger (Variables|Default|GetSpawn_Chance)) 0)
          (bind _returnvalue (Game|SpawnActorfromClass "/Game/Blueprints/Mob_Re_Blueprint.Mob_Re_Blueprint_C" (Math|Transform|MakeTransform (Math|Vector|MakeVector (Math|Random|RandomFloatinRange -2.5e+03 3.1e+03) 387.0 3178.0) "0, 0, 0" "1,1,1") "Undefined" 0 0))
          (Audio|PlaySoundatLocation "/Game/Sounds/Balloon_Start_Sound.Balloon_Start_Sound" (Transformation|GetActorLocation _returnvalue) "0, 0, 0" 0.4 (Math|Random|RandomFloatinRange 0.8 1.2)))))))

(event Input|KeyboardEvents|AnyKey
  (params (Key :type Key%20Structure :default "AnyKey"))
  ;[1 1 1] 키 이벤트 전달
  (:Pressed
    (if (not (Variables|Default|GetIsGameOver))
      (if (== Key "Escape")
        (CallFunction|Pause)
        (else
          (for _array_element (Variables|Default|GetMob_Re)
            (Default|KeyPressed _array_element Key))
          ;[1 1 1] 풍선에 있는 글자를 쳤는가?
          (if (> 0 (Variables|Default|GetSuccess_Count))
            ;[1 1 1] 벌칙-낙하 속도 증가
            (Audio|PlaySound2D "/Game/Sounds/Wrong_Sound.Wrong_Sound" 1.0 1.0)
            (Variables|Default|SetFall_Speed (+ 0.2 (Variables|Default|GetFall_Speed)))
            (Default|SpeedUpdate (Variables|Widgets|GetDefault_Widget) 0.2 "Wrong Key")
            (else
              (Utilities|Array|Clear (Variables|Default|GetMob_Re))
              (Variables|Default|SetSuccess_Count -1))))))))

(fn ConstructionScript)